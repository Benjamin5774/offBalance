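; BP_CameraFollower is an actor that moves itself to the player camera's location every tick.
; BeginPlay caches player 0's camera manager and the pawn's static mesh component, though the cached mesh is never read.
; Tick copies the camera location without sweep or rotation, then prints that location, the view target's name and the pawn mesh's world location for debugging.
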(event Collision|EventActorBeginOverlap
  (params (OtherActor :type Actor%20Object%20Reference)))

(event EventBeginPlay
  (Variables|Default|SetPCM (Variables|/Script/Engine.PlayerController|GetPlayerCameraManager (Game|GetPlayerController 0)))
  (Variables|Default|SetFollowComponent (Actor|GetComponentbyClass (Game|Player|GetPlayerPawn 0) "/Script/Engine.StaticMeshComponent")))

(event EventTick
  (params (DeltaSeconds :type Float%20%28single-precision%29))
  (bind _pcm (Variables|Default|GetPCM))
  (Utilities|FlowControl|Sequence
    (:then_0
      (if (Utilities|IsValid _pcm)
        (Transformation|SetActorLocation (Camera|GetCameraLocation _pcm) false false)
        (Development|PrintString (Utilities|String|ToString(Vector) (Camera|GetCameraLocation (Variables|Default|GetPCM))))))
    (:then_1
      (Development|PrintString (Utilities|GetDisplayName (Pawn|GetViewTarget (Game|GetPlayerController 0)))))
    (:then_2
      (Development|PrintString (Utilities|String|ToString(Vector) (Transformation|GetWorldLocation (Actor|GetComponentbyClass (Game|Player|GetPlayerPawn 0) "/Script/Engine.StaticMeshComponent")))))))

(fn ConstructionScript)