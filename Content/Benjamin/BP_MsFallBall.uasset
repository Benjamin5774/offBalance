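; BP_MsFallBall is a ball game Blueprint steered by roll and pitch values read from an OCR reference.
; Each tick it applies a small offset and gain to both, feeding the result to MovementComponent as movement input and to SetSwayInput to rock the board.
; BeginPlay registers Camera as the sway camera.
; An older serial-port path that parsed angular readings into movement is abandoned and never runs.
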(event Custom|SerialUpdate1
  ;[0.15 0.15 0.15 0.5] 废案
)

(event EventTick
  (params (DeltaSeconds :type Float%20%28single-precision%29))
  (bind _ocr (Variables|Default|GetOCR))
  (bind _fpitch (Variables|/Game/Benjamin/OCR.OCR_C|GetFPitch _ocr))
  (bind _froll (Variables|/Game/Benjamin/OCR.OCR_C|GetFRoll _ocr))
  (bind _returnvalue (+ _froll 0.004))
  (bind _returnvalue_2 (+ _fpitch 0.0))
  (bind _returnvalue_3 (* _returnvalue 2.0))
  (bind _returnvalue_4 (* _returnvalue_2 2.0))
  (bind _returnvalue_5 (Math|Vector|MakeVector _returnvalue_3 _returnvalue_4 0.0))
  (Utilities|FlowControl|Sequence
    (:then_0
      ;[0.15 0.15 0.15 0.5] 传入速度
      (Class|MsFallBallMovementComponent|AddMovementInput (Variables|Default|GetMovementComponent) (Math|Conversions|ToVector2D(Vector) _returnvalue_5))
      ;[0.15 0.15 0.15 0.5] 摇晃船板
      (Class|MsFallBall|SetSwayInput (Math|Conversions|ToVector2D(Vector) (* _returnvalue_5 "1.000000,1.000000,0.000000"))))))

(event EventBeginPlay
  ;[0.15 0.15 0.15 0.5] 传入摄像机
  (Class|MsFallBall|SetSwayCamera (Variables|Default|GetCamera)))

(fn ConstructionScript)