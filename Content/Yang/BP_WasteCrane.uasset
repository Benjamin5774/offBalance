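; BP_WasteCrane is a claw crane that grabs, holds and releases the player's BP_MsFallBall pawn.
; Grab and Release events play timelines that pitch four crane meshes by a scaled angle to close or open the claw.
; BindBall2Crane starts a Tick that teleports the ball to HoldPosition, with physics switched off through a DoOnce.
; Release stops that binding, then resets the DoOnce and restores ball physics when its timeline finishes.
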(event Custom|Grab
  ;[0.15 0.15 0.15 0.5] Grab And Release
  (bind _rota (Timeline|GrabTimeLine PlayFromStart)
    (:Update
      (Variables|Default|SetDegreeUpdate _rota)
      (Utilities|SetCraneDegrees))))

(event Custom|Release
  ;[0.15 0.15 0.15 0.5] Grab And Release
  (Variables|Default|SetIsBinding false)
  (bind _rota (Timeline|ReleaseTimeLine Play)
    (:Update
      (Variables|Default|SetDegreeUpdate _rota)
      (Utilities|SetCraneDegrees))
    (:Finished
      (Utilities|FlowControl|Sequence
        (:then_0
          ;[0.15 0.15 0.15 0.5] Bind
          (Utilities|FlowControl|DoOnce false) ; enters at Reset
        )
        (:then_1
          (Physics|SetSimulatePhysics (Variables|/Script/OffBalance.MsFallBall|GetBallMesh (stale EventTick _asbp_ms_fall_ball)) true))))))

(event Custom|BindBall2Crane
  ;[0.15 0.15 0.15 0.5] Bind
  (Variables|Default|SetPlayerCache (Game|Player|GetPlayerPawn 0))
  (Variables|Default|SetIsBinding true))

(event Collision|EventActorBeginOverlap
  (params (OtherActor :type Actor%20Object%20Reference)))

(event EventTick
  (params (DeltaSeconds :type Float%20%28single-precision%29))
  ;[0.15 0.15 0.15 0.5] Bind
  (if (Variables|Default|GetIsBinding)
    (bind _asbp_ms_fall_ball (Utilities|Casting|CastToBP_MsFallBall (Variables|Default|GetPlayerCache)))
    (Utilities|FlowControl|Sequence
      (:then_0
        (Utilities|FlowControl|DoOnce false
          (:Completed
            (Physics|SetSimulatePhysics (Variables|/Script/OffBalance.MsFallBall|GetBallMesh _asbp_ms_fall_ball) false))))
      (:then_1
        (Transformation|SetWorldLocation (Variables|/Script/OffBalance.MsFallBall|GetBallMesh _asbp_ms_fall_ball) (Transformation|GetWorldLocation (Variables|Default|GetHoldPosition)) false true)))))

(fn ConstructionScript)