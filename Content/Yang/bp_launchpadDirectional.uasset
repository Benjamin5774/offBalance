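; Directional launchpad that propels MrBall or BP_MsFallBall when either overlaps its Trigger.
; MrBall is launched as a Character using CalculateForce2, while BP_MsFallBall's physics mesh has its velocity replaced by DirectionVelocity, then receives force from CalculateForce.
; Both helper graphs contain Arrow-forward math scaled by LaunchForce at different magnitudes, but that math appears unused.
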(event OnComponentBeginOverlap(trigger)
  (params (OverlappedComponent :type Primitive%20Component%20Object%20Reference) (OtherActor :type Actor%20Object%20Reference) (OtherComp :type Primitive%20Component%20Object%20Reference) (OtherBodyIndex :type Integer) (bFromSweep :type Boolean) (SweepResult :type Hit%20Result%20Structure%20%28by%20ref%29))
  (bind _asmr_ball (Utilities|Casting|CastToMrBall OtherActor)
    (:then
      (Character|LaunchCharacter _asmr_ball (|CalculateForce2) false false))
    (:CastFailed
      (bind _asbp_ms_fall_ball (Utilities|Casting|CastToBP_MsFallBall OtherActor))
      (Physics|SetPhysicsLinearVelocity (Variables|/Script/OffBalance.MsFallBall|GetBallMesh _asbp_ms_fall_ball) (Variables|Default|Getdirection%20velocity) false "None")
      (Physics|AddForce (Variables|/Script/OffBalance.MsFallBall|GetBallMesh _asbp_ms_fall_ball) (|CalculateForce) "None" false))))

(event EventBeginPlay)

(event Collision|EventActorBeginOverlap
  (params (OtherActor :type Actor%20Object%20Reference)))

(event EventTick
  (params (DeltaSeconds :type Float%20%28single-precision%29)))

(fn ConstructionScript)