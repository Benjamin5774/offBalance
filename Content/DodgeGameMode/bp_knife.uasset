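; Swinging knife hazard for the dodge game mode that knocks out the player on contact.
; On BeginPlay the Swing timeline drives the roll of the Scene component, scaled by Maxangle, with sweep enabled.
; When Collision overlaps the third-person character, it ragdolls the mesh, disables movement and opens ThirdPersonMap after a short delay.
; An explosion-and-destroy chain is present but never runs.
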(event OnComponentBeginOverlap(collision)
  (params (OverlappedComponent :type Primitive%20Component%20Object%20Reference) (OtherActor :type Actor%20Object%20Reference) (OtherComp :type Primitive%20Component%20Object%20Reference) (OtherBodyIndex :type Integer) (bFromSweep :type Boolean) (SweepResult :type Hit%20Result%20Structure%20%28by%20ref%29))
  (bind _asbp_third_person_character (Utilities|Casting|CastToBP_ThirdPersonCharacter OtherActor))
  (Physics|SetSimulatePhysics (Variables|/Script/Engine.Character|GetMesh _asbp_third_person_character) true)
  (Collision|SetCollisionProfileName (Variables|/Script/Engine.Character|GetMesh _asbp_third_person_character) "Ragdoll" true :!class /Script/Engine.PrimitiveComponent)
  (Pawn|Components|CharacterMovement|DisableMovement (Variables|/Script/Engine.Character|GetCharacterMovement _asbp_third_person_character))
  (Utilities|FlowControl|Delay 3.0)
  (Game|OpenLevel(byName) "ThirdPersonMap"))

(event EventBeginPlay
  (bind _alpha (Timeline|swing Play)
    (:Update
      (Transformation|SetRelativeRotation (Variables|Default|GetScene) (Math|Rotator|MakeRotator (* _alpha (Variables|Default|Getmaxangle)) 0.0 0.0) true false))))

(event Collision|EventActorBeginOverlap
  (params (OtherActor :type Actor%20Object%20Reference)))

(event EventTick
  (params (DeltaSeconds :type Float%20%28single-precision%29)))

(fn ConstructionScript)