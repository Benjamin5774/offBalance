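; Piston actor for the dodge game mode that extends a moving part and retracts it, repeating automatically when AutoPush is enabled.
; The Push event plays a timeline that drives MovePartRoot's relative Z, scaled by PushLength, waits HoldTime, then plays a separate reverse timeline.
; The auto loop re-triggers Push after a delay summing push duration, hold time and a hard-coded margin, independent of timeline completion.
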(event Custom|Push
  (bind _pushtimeline (Timeline|PushTimeLine PlayFromStart)
    (:Update
      (Variables|Default|SetRelativeLocationUpdate _pushtimeline))
    (:Finished
      (Utilities|FlowControl|Delay (Variables|Default|GetHoldTime))
      (bind _reversetimeline (Timeline|ReverseTimeline PlayFromStart)
        (:Update
          (Variables|Default|SetRelativeLocationUpdate _reversetimeline)))))
  (Transformation|SetRelativeLocation (Variables|Default|GetMovePartRoot) (Math|Vector|MakeVector 0.0 0.0 (* (Variables|Default|GetRelativeLocationUpdate) 1e+02 (Variables|Default|GetPushLength))) false false))

(event EventBeginPlay
  (if (Variables|Default|GetAutoPush)
    (CallFunction|Push :!label _label)
    (Utilities|FlowControl|Delay (+ (Variables|Default|GetPushDuation) (Variables|Default|GetHoldTime) 0.4))
    (goto _label)))

(event Collision|EventActorBeginOverlap
  (params (OtherActor :type Actor%20Object%20Reference)))

(event EventTick
  (params (DeltaSeconds :type Float%20%28single-precision%29)))

(fn ConstructionScript)