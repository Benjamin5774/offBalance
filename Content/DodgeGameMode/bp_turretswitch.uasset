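; Turret switch actor in the dodge game mode that lets the player shut down a linked turret.
; It enables input on BeginPlay, and pressing E while the player character overlaps its trigger box sets the target turret's disabled flag.
; The switch mesh then swaps to a basic wall material, with no path to re-enable the turret.
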(event EventBeginPlay
  (Input|EnableInput (Game|GetPlayerController 0)))

(event Input|KeyboardEvents|E
  (params (Key :type Key%20Structure))
  (:Pressed
    (if (Collision|IsOverlappingActor (Variables|Default|GetBox1) (Game|GetPlayerCharacter 0) :!class /Script/Engine.PrimitiveComponent)
      (Variables|/Game/DodgeGameMode/bp_turret.bp_turret_C|SetbIsDisabled (Variables|Default|GetTargetTurret) true)
      (Rendering|Material|SetMaterial (Variables|Default|Getbox) 0 "/Game/StarterContent/Materials/M_Basic_Wall.M_Basic_Wall"))))

(fn ConstructionScript)